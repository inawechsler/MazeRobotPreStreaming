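; Enemy drone that detects the player inside its sphere and resets at its spawn point when the player dies.
; Sphere overlap flags detection on the BT_Dron blackboard if the player moves or stands with clear line of sight.
; CheckTimeDetected kills the player after a retriggerable delay, but its timer and those for sight and range checks are unconnected.
; Death, bound every Tick to the player's death event, destroys and respawns the drone.
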(event `Death`
  (set `self.Died` true)
  (bind _asaic_dron (cast `/Game/Enemy/AIC_Dron` (`AIBlueprintHelperLibrary.GetAIController` self)))
  (`/Game/Enemy/AIC_Dron.Death` _asaic_dron)
  (`self.K2_DestroyActor`)
  (set `self.Died` false)
  (`AIBlueprintHelperLibrary.SpawnAIFromClass` "BP_ENMYDRONE_C" "/Game/Enemy/BT_Dron.BT_Dron" (`self.SpawnPos`) (struct) false null))

(event `CheckTimeDetected`
  (if (`/Game/ThirdPerson/Blueprints/BP_ThirdPersonCharacter.IsDead` (`self.PlayerRef`))
    _
    (elif (not (`self.PJIsDetected`))
      (`KismetSystemLibrary.RetriggerableDelay` 2.9)
      (if (`self.PJIsDetected`)
        (`/Game/ThirdPerson/Blueprints/BP_ThirdPersonCharacter.Death` (`self.PlayerRef`))))))

(event `self.ReceiveTick`
  (params (DeltaSeconds :type "Float (single-precision)"))
  (bind _returnvalue (+ (`self.Duration_0`) 0.014))
  (add `/Game/ThirdPerson/Blueprints/BP_ThirdPersonCharacter.SetIsDead` (`self.PlayerRef`) (delegate `Death`))
  (if (`self.PJIsDetected`)
    (bind _output_get (set `self.Duration_0` _returnvalue))
    (if (not (>= _returnvalue 3.02))
      (`KismetSystemLibrary.PrintString` (`KismetStringLibrary.Conv_DoubleToString` _output_get)))
    (else
      (set `self.Duration_0` 0.0))))

(event `self.Sphere.OnComponentBeginOverlap`
  (params (OverlappedComponent :type "PrimitiveComponent Object Reference") (OtherActor :type "Actor Object Reference") (OtherComp :type "PrimitiveComponent Object Reference") (OtherBodyIndex :type Integer) (bFromSweep :type Boolean) (SweepResult :type "HitResult Structure (by ref)"))
  (bind _playerref (`self.PlayerRef`))
  (if (== OtherActor (`self.PlayerRef`))
    (if (or (`/Game/ThirdPerson/Blueprints/BP_ThirdPersonCharacter.IsMoving` _playerref) (not (`Character.bIsCrouched` _playerref))) :!label _label
      (if (`self.Blocking Hit`) :!label _label_2
        (`KismetSystemLibrary.Delay` 0.2)
        (if (`self.InsideSphere`)
          (goto _label_2))
        (else
          (set `self.PJIsDetected` true)
          (`BlackboardComponent.SetValueAsBool` (`AIBlueprintHelperLibrary.GetBlackboard` null) "IsDetecting" true)))
      (else
        (`KismetSystemLibrary.Delay` 0.2)
        (if (`self.InsideSphere`)
          (goto _label))))))

(event `self.ReceiveBeginPlay`
  (set `self.SpawnPos` (`self.K2_GetActorLocation`))
  (bind _returnvalue (`GameplayStatics.GetActorOfClass` "/Game/ThirdPerson/Blueprints/BP_ThirdPersonCharacter.BP_ThirdPersonCharacter_C"))
  (set `self.PlayerRef` _returnvalue)
  (`KismetSystemLibrary.PrintString` "Hello"))

(event `RayToChar`
  (bind _playerref (`self.PlayerRef`))
  (if (not (`/Game/ThirdPerson/Blueprints/BP_ThirdPersonCharacter.IsDead` _playerref))
    (bind _outhit (`KismetSystemLibrary.LineTraceSingle` (+ (`self.K2_GetActorLocation`) (0.0 0.0 1095.0)) (`SceneComponent.K2_GetComponentLocation` (`Character.Mesh` _playerref)) "TraceTypeQuery1"))
    (set `self.Blocking Hit` (`GameplayStatics.BreakHitResult` _outhit))))

(event `self.Sphere.OnComponentEndOverlap`
  (params (OverlappedComponent :type "PrimitiveComponent Object Reference") (OtherActor :type "Actor Object Reference") (OtherComp :type "PrimitiveComponent Object Reference") (OtherBodyIndex :type Integer))
  (if (== OtherActor (`self.PlayerRef`))
    (if (`self.Blocking Hit`)
      _
      (elif true
        (set `self.PJIsDetected` false)
        (`BlackboardComponent.SetValueAsBool` (`AIBlueprintHelperLibrary.GetBlackboard` null) "IsDetecting" false)))))

(fn `CheckPlayerOnSphere`
  (bind _playerref (`self.PlayerRef`))
  (bind _sphereradius (`SphereComponent.SphereRadius` (`self.Sphere`)))
  (if (not (`/Game/ThirdPerson/Blueprints/BP_ThirdPersonCharacter.IsDead` _playerref))
    (set `self.InsideSphere` (< (`KismetMathLibrary.Vector_Distance` (`SceneComponent.K2_GetComponentLocation` (`self.Sphere`)) (`SceneComponent.K2_GetComponentLocation` (`Character.Mesh` _playerref))) (+ _sphereradius (/ _sphereradius 4.0))))))

(fn `Get Next Array Point`
  (for (_array_element _array_index) (`self.DronWP`)
    (set `self.Array Index` _array_index)
    (set `self.NewVar_0` (`self.K2_GetActorLocation` _array_element))))

(fn `RayToCharacter`
  (if (not (`/Game/ThirdPerson/Blueprints/BP_ThirdPersonCharacter.IsDead` (`self.PlayerRef`)))
    (bind _outhit (`KismetSystemLibrary.LineTraceSingle` (+ (`self.K2_GetActorLocation`) (0.0 0.0 1095.0)) (`SceneComponent.K2_GetComponentLocation` (`Character.Mesh` (`self.PlayerRef`))) "TraceTypeQuery1"))
    (set `self.Blocking Hit` (`GameplayStatics.BreakHitResult` _outhit))))

(fn `UserConstructionScript`)