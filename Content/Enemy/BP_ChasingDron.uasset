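; Enemy drone that kills the player character when it overlaps the drone's sphere; no movement logic for chasing appears in its graphs.
; A timer set at BeginPlay runs ManagePos, which jumps the drone once to a preset location if the player is speed-boosted.
; The drone binds to the player's SetIsDead dispatcher every Tick, teleporting back to its saved spawn position when that fires.
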(event `Death`
  (`self.K2_TeleportTo` (`self.SpawnPos`)))

(event `self.ReceiveTick`
  (params (DeltaSeconds :type "Float (single-precision)"))
  (add `/Game/ThirdPerson/Blueprints/BP_ThirdPersonCharacter.SetIsDead` (`self.As BP Third Person Character`) (delegate `Death`)))

(event `ManagePos`
  (if (`/Game/ThirdPerson/Blueprints/BP_ThirdPersonCharacter.IsOnSpeedBoost` (`self.As BP Third Person Character`))
    (`/Engine/EditorBlueprintResources/StandardMacros.DoOnce` false
      (:`Completed`
        (`KismetSystemLibrary.PrintString` "Entre")
        (`self.K2_SetActorLocation` (`self.New Location`))
        (set `self.Looping` false)))))

(event `self.ReceiveBeginPlay`
  (set `self.SpawnPos` (`self.K2_GetActorLocation`))
  (bind _asbp_third_person_character (cast `/Game/ThirdPerson/Blueprints/BP_ThirdPersonCharacter` (`GameplayStatics.GetPlayerCharacter` 0)))
  (set `self.As BP Third Person Character` _asbp_third_person_character)
  (`KismetSystemLibrary.K2_SetTimerDelegate` (delegate `ManagePos`) 0.2 (`self.Looping`)))

(event `self.Sphere.OnComponentBeginOverlap`
  (params (OverlappedComponent :type "PrimitiveComponent Object Reference") (OtherActor :type "Actor Object Reference") (OtherComp :type "PrimitiveComponent Object Reference") (OtherBodyIndex :type Integer) (bFromSweep :type Boolean) (SweepResult :type "HitResult Structure (by ref)"))
  (bind _as_bp_third_person_character (`self.As BP Third Person Character`))
  (if (== OtherActor _as_bp_third_person_character)
    (`/Game/ThirdPerson/Blueprints/BP_ThirdPersonCharacter.Death` _as_bp_third_person_character)))

(fn `UserConstructionScript`)