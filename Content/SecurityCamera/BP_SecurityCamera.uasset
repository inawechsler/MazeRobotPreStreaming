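; Security camera that sweeps an area and kills the player inside its detection cone unless they are crouched and still.
; A looping timer drives ManageCamera, where nested FlipFlops pick 45-degree yaw steps, RInterpTo turns the camera, and a delay gates each step, with a proximity-based sound.
; Throwable hits on the capsule set Desactivate for five seconds, alternately spawning steam or turning off cone tick.
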(event `self.ReceiveBeginPlay`
  (bind _asbp_third_person_character (cast `/Game/ThirdPerson/Blueprints/BP_ThirdPersonCharacter` (`GameplayStatics.GetPlayerCharacter` 0)))
  (set `self.Player` _asbp_third_person_character)
  (`KismetSystemLibrary.K2_SetTimerDelegate` (delegate `ManageCamera`) 0.01 true))

(event `ManageCamera`
  (bind _camera (`self.Camera`))
  (bind _player (`self.Player`))
  (bind (_returnvalue_roll _returnvalue_pitch _returnvalue_yaw) (`KismetMathLibrary.BreakRotator` (`SceneComponent.K2_GetComponentRotation` (`self.Camera`))))
  (bind _returnvalue_x (`KismetMathLibrary.BreakVector` (`KismetMathLibrary.Conv_RotatorToVector` (`KismetMathLibrary.NormalizedDeltaRotator` (`SceneComponent.K2_GetComponentRotation` (`self.Camera`)) (`self.TargetRotation`)))))
  (bind _returnvalue (`KismetMathLibrary.Vector_Distance` (`SceneComponent.K2_GetComponentLocation` (`Character.CapsuleComponent` (`GameplayStatics.GetPlayerCharacter` 0))) (`SceneComponent.K2_GetComponentLocation` (`self.Camera`))))
  (if (`self.Desactivate`)
    (`/Engine/EditorBlueprintResources/StandardMacros.DoOnce` false
      (:`Completed`
        (`KismetSystemLibrary.PrintString` "Desactivada")))
    (elif (`self.IsInArea`)
      (if (and (not (`/Game/ThirdPerson/Blueprints/BP_ThirdPersonCharacter.IsMoving` (`self.Player`))) (`Character.bIsCrouched` _player))
        (`|ExecutionSequence` :!label _label
          (:`then_0`
            (`/Engine/EditorBlueprintResources/StandardMacros.DoOnce` false :!label _label_2
              (:`Completed`
                (`/Engine/EditorBlueprintResources/StandardMacros.FlipFlop`
                  (:`A`
                    (`/Engine/EditorBlueprintResources/StandardMacros.FlipFlop`
                      (:`A`
                        (set `self.TargetRotation` (`KismetMathLibrary.MakeRotator` _returnvalue_roll _returnvalue_pitch (+ _returnvalue_yaw 45.0)) :!label _label_3))
                      (:`B`
                        (set `self.TargetRotation` (`KismetMathLibrary.MakeRotator` _returnvalue_roll _returnvalue_pitch (+ _returnvalue_yaw -45.0)) :!label _label_4))))
                  (:`B`
                    (`/Engine/EditorBlueprintResources/StandardMacros.FlipFlop`
                      (:`A`
                        (goto _label_4))
                      (:`B`
                        (goto _label_3)))))
                (if (< _returnvalue 1600.0)
                  (`GameplayStatics.PlaySoundAtLocation` "/Game/ThirdPerson/FX/SFX/CamSfx.CamSfx" (0.0 0.0 0.0) (struct) 0.4 1.0 0.0 null null null null)
                  (else
                    (`KismetSystemLibrary.PrintString` (`KismetStringLibrary.Conv_DoubleToString` _returnvalue)))))))
          (:`then_1`
            (`SceneComponent.K2_SetWorldRotation` _camera (`KismetMathLibrary.RInterpTo` (`SceneComponent.K2_GetComponentRotation` _camera) (`self.TargetRotation`) (`GameplayStatics.GetWorldDeltaSeconds`) (`self.RotationSpeed`)) false false)
            (if (> _returnvalue_x 0.9)
              (`KismetSystemLibrary.Delay` 4.0)
              (goto _label_2 :!via `Reset`))))
        (else
          (`/Engine/EditorBlueprintResources/StandardMacros.DoOnce` false
            (:`Completed`
              (`/Game/ThirdPerson/Blueprints/BP_ThirdPersonCharacter.Death` _player)))))
      (else
        (goto _label)))))

(event `self.Cone.OnComponentBeginOverlap`
  (params (OverlappedComponent :type "PrimitiveComponent Object Reference") (OtherActor :type "Actor Object Reference") (OtherComp :type "PrimitiveComponent Object Reference") (OtherBodyIndex :type Integer) (bFromSweep :type Boolean) (SweepResult :type "HitResult Structure (by ref)"))
  (if (`ActorComponent.ComponentHasTag` OtherComp "Player")
    (set `self.DetectedActor` OtherActor)
    (set `self.IsInArea` true)))

(event `self.Cone.OnComponentEndOverlap`
  (params (OverlappedComponent :type "PrimitiveComponent Object Reference") (OtherActor :type "Actor Object Reference") (OtherComp :type "PrimitiveComponent Object Reference") (OtherBodyIndex :type Integer))
  (cast `/Game/ThirdPerson/Blueprints/BP_ThirdPersonCharacter` OtherActor)
  (set `self.IsInArea` false))

(event `self.Capsule.OnComponentBeginOverlap`
  (params (OverlappedComponent :type "PrimitiveComponent Object Reference") (OtherActor :type "Actor Object Reference") (OtherComp :type "PrimitiveComponent Object Reference") (OtherBodyIndex :type Integer) (bFromSweep :type Boolean) (SweepResult :type "HitResult Structure (by ref)"))
  (if (`self.ActorHasTag` OtherActor "Throwable")
    (set `self.Desactivate` true)
    (`/Engine/EditorBlueprintResources/StandardMacros.FlipFlop`
      (:`A`
        (bind _returnvalue (`GameplayStatics.SpawnEmitterAtLocation` "/Game/StarterContent/Particles/P_Steam_Lit.P_Steam_Lit" (`SceneComponent.K2_GetComponentLocation` (`self.Camera`)) (struct) (2.0 2.0 2.0)))
        (`KismetSystemLibrary.Delay` 5.0)
        (`ActorComponent.K2_DestroyComponent` _returnvalue))
      (:`B`
        (`ActorComponent.SetComponentTickEnabled` (`self.Cone`) false)
        (`KismetSystemLibrary.Delay` 5.0)))
    (set `self.Desactivate` false)))

(fn `UserConstructionScript`)