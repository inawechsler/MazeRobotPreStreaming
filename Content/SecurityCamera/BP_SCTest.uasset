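; BP_SCTest is a test security camera that sweeps its view back and forth along a spline.
; BeginPlay starts Sweep, a self-calling event that uses a macro to aim the camera at the current spline distance, then advances it by MoveDelta.
; At either spline end it reverses MoveDelta and pauses briefly; intermediate steps recurse with no delay.
; An unconnected MoveComponentTo node never runs.
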(event `self.ReceiveBeginPlay`
  (`self.Sweep`))

(event `Sweep`
  (bind _movedelta (`self.MoveDelta`))
  (bind _returnvalue (+ (`self.Distance`) _movedelta))
  (`self.NewMacro` (`self.Distance`))
  (if (> _returnvalue (`SplineComponent.GetSplineLength` (`self.Spline`)))
    (bind _output_get (set `self.MoveDelta` (* _movedelta -1.0) :!label _label))
    (`KismetSystemLibrary.Delay` 3.0)
    (elif (< _returnvalue 0.0)
      (goto _label)
      (else
        _)))
  (set `self.Distance` (+ _output_get (`self.Distance`)))
  (`self.Sweep`))

(fn `UserConstructionScript`)